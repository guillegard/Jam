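; BP_Chest is an interactable chest that opens and closes with sound and a gold glow.
; Interact branches on IsOpen, playing the OpenTreasure timeline after a one-second delay to open, or hiding the glow and reversing it immediately to close.
; The timeline rotates the lid.
; On finish, a FlipFlop alternates between setting IsOpen with the glow shown and clearing IsOpen, rather than checking playback direction.
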(event EventBeginPlay
  (|CallParentFunction))

(event Collision|EventActorBeginOverlap
  (params (OtherActor :type Actor%20Object%20Reference))
  (|CallParentFunction OtherActor) ; This node is disabled and will not be called.\nDrag off pins to build functionality.
)

(event EventTick
  (params (DeltaSeconds :type Float%20%28single-precision%29))
  (|CallParentFunction DeltaSeconds) ; This node is disabled and will not be called.\nDrag off pins to build functionality.
)

(event EventInteract
  (bind _staticmesh (Variables|Default|GetStaticMesh))
  (bind _returnvalue (Transformation|GetWorldLocation _staticmesh))
  (if (Variables|Default|GetIsOpen?)
    (Audio|PlaySoundatLocation "/Game/SFX/Chest/OpenRealChest.OpenRealChest" _returnvalue "0, 0, 0" 1.0 1.0 0.0 0 0 0)
    (Rendering|SetVisibility (Variables|Default|GetGoldGlow) false false)
    (bind _topopenangle (Timeline|Open%20Treasure Reverse)
      (:Update
        (Transformation|SetRelativeRotation (Variables|Default|GetchestLid_low) (Math|Rotator|MakeRotator 0.0 _topopenangle 0.0) false false))
      (:Finished
        (Utilities|FlowControl|FlipFlop
          (:A
            (Variables|Default|SetIsOpen? true)
            (Rendering|SetVisibility (Variables|Default|GetGoldGlow) true false))
          (:B
            (Variables|Default|SetIsOpen? false)))))
    (else
      (Audio|PlaySoundatLocation "/Game/SFX/Chest/OpenRealChest.OpenRealChest" _returnvalue "0, 0, 0" 1.0 1.0 0.0 0 0 0)
      (Utilities|FlowControl|Delay 1.0)
      (Timeline|Open%20Treasure Play))))

(fn ConstructionScript
  (|CallParentFunction))