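; Master Blueprint for a mana potion pickup that restores mana to the player when interacted with.
; Interact calls IncreaseMana on the player reference with the potion's mana value, spawns a Niagara effect at the mesh's location and rotation, then destroys the actor.
; The construction script applies a material variable to the static mesh, so the potion's look can vary.
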(event EventBeginPlay
  (|CallParentFunction) ; This node is disabled and will not be called.\nDrag off pins to build functionality.
)

(event Collision|EventActorBeginOverlap
  (params (OtherActor :type Actor%20Object%20Reference))
  (|CallParentFunction OtherActor) ; This node is disabled and will not be called.\nDrag off pins to build functionality.
)

(event EventTick
  (params (DeltaSeconds :type Float%20%28single-precision%29))
  (|CallParentFunction DeltaSeconds) ; This node is disabled and will not be called.\nDrag off pins to build functionality.
)

(event EventInteract
  (bind _staticmesh (Variables|Default|GetStaticMesh))
  (bind _returnvalue (Transformation|GetWorldTransform _staticmesh))
  (Class|JamCharacter|IncreaseMana (Variables|Default|GetPlayer%20Ref) (Variables|Default|GetMana%20Value))
  (Niagara|SpawnSystematLocation (Variables|Default|GetNiagaraSystem) (.location _returnvalue) (.rotation _returnvalue))
  (Actor|DestroyActor))

(fn ConstructionScript
  (|CallParentFunction)
  (Rendering|Material|SetMaterial (Variables|Default|GetStaticMesh) 0 (Variables|Default|GetMaterial)))